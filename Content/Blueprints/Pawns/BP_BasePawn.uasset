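; BP_BasePawn is a base pawn that can take damage and fire projectiles.
; AnyDamage forwards the damage amount to its Health component.
; The Fire event spawns BP_Projectile at SpawnPoint's transform, using a boolean and a Delay as a one-second cooldown.
; OnActorDeath is an empty function, and destruction only prints a debug message.
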(event Custom|Event%20Fire
  ;[1 1 1] Fire Event
  (if (not (Variables|Default|GetIs%20Fire%20On%20Cooldown))
    (Variables|Default|SetIs%20Fire%20On%20Cooldown true)
    (Game|SpawnActorfromClass "/Game/Blueprints/BP_Projectile.BP_Projectile_C" (Transformation|GetWorldTransform (Variables|Default|GetSpawn%20Point)) "AlwaysSpawn" "OverrideRootScale" 0 0)
    (Utilities|FlowControl|Delay 1.0)
    (Variables|Default|SetIs%20Fire%20On%20Cooldown false)))

(event EventBeginPlay)

(event Collision|EventActorBeginOverlap
  (params (OtherActor :type Actor%20Object%20Reference)))

(event EventTick
  (params (DeltaSeconds :type Float%20%28single-precision%29)))

(event Game|Damage|EventAnyDamage
  (params (Damage :type Float%20%28single-precision%29) (DamageType :type Damage%20Type%20Object%20Reference) (InstigatedBy :type Controller%20Object%20Reference) (DamageCauser :type Actor%20Object%20Reference))
  (Default|OnTakeAnyDamage (Variables|Default|GetHealth) Damage))

(event EventDestroyed
  (Development|PrintString "Destroyed"))

(fn ConstructionScript)

(fn OnActorDeath)