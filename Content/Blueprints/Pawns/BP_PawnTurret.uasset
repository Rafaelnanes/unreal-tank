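; BP_PawnTurret is an enemy turret pawn that tracks and fires at the player's tank.
; Each Tick it checks distance to the player; when in range, it yaws its capsule toward the tank and line-traces to confirm line of sight.
; A looping one-second timer calls the fire event only while both checks pass.
; An alternative delay-gated debug firing block is left unconnected.
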(event Custom|Event%20Turret%20Fire
  ;[1 1 1] Fire Projectile
  (if (and (Variables|Default|GetIs%20In%20Range) (Variables|Default|GetIs%20Pawn%20On%20Trace))
    (CallFunction|EventFire)))

(event EventBeginPlay
  ;[1 1 1] Begin
  (|CallParentFunction)
  (Variables|Default|SetMissle%20Max%20Distance 5e+02)
  (bind _asbp_pawn_tank (Utilities|Casting|CastToBP_PawnTank (Game|Player|GetPlayerPawn 0)))
  (Variables|Default|SetPlayer _asbp_pawn_tank)
  (Utilities|Time|SetTimerbyEvent (delegate Custom|Event%20Turret%20Fire) 1.0 true))

(event EventTick
  (params (DeltaSeconds :type Float%20%28single-precision%29))
  (bind _returnvalue (Transformation|GetActorLocation))
  (bind _player (Variables|Default|GetPlayer))
  (bind _returnvalue_2 (Transformation|GetActorLocation _player))
  (|CallParentFunction DeltaSeconds)
  ;[1 1 1] Turret Look At
  (bind _output_get (Variables|Default|SetIs%20In%20Range (<= (Math|Vector|Distance(Vector) _returnvalue _returnvalue_2) (Variables|Default|GetDistance%20Range))))
  (if _output_get
    (Transformation|SetWorldRotation (Variables|Default|GetCollision%20Capsule) (Math|Rotator|MakeRotator 0.0 0.0 (.Yaw (Math|Rotator|BreakRotator (Math|Rotator|FindLookatRotation _returnvalue _returnvalue_2)))) false false)
    ;[1 1 1] Is Pawn The Target?
    (bind _outhit (Collision|LineTraceForObjects (Transformation|GetWorldLocation (Variables|Default|GetCollision%20Capsule)) (Transformation|GetActorLocation (Variables|Default|GetPlayer)) (Utilities|Array|MakeArray "ObjectTypeQuery3" "ObjectTypeQuery1") false 0 "None" true "(R=1.000000,G=0.000000,B=0.000000,A=1.000000)" "(R=0.000000,G=1.000000,B=0.000000,A=1.000000)" 0.0))
    (Variables|Default|SetIs%20Pawn%20On%20Trace (Utilities|ClassIsChildOf (Utilities|GetClass (.hitactor _outhit)) "/Game/Blueprints/Pawns/BP_PawnTank.BP_PawnTank_C"))))

(fn ConstructionScript
  (|CallParentFunction))