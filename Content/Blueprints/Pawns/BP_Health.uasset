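; BP_Health is a health component that tracks a pawn's health, updates its health bar and destroys it at zero.
; On BeginPlay it caches its owner as BP_BasePawn if the class matches.
; OnTakeAnyDamage gets the pawn's BP_WG_HealthBar widget, subtracts damage from Amount and sends the result divided by 100 to the widget.
; It then destroys the pawn once Amount reaches zero or below.
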(event EventBeginPlay
  (bind _returnvalue (Components|GetOwner))
  ;[1 1 1] Set Base Pawn
  (if (Utilities|ClassIsChildOf (Utilities|GetClass _returnvalue) "/Game/Blueprints/Pawns/BP_BasePawn.BP_BasePawn_C")
    (bind _asbp_base_pawn (Utilities|Casting|CastToBP_BasePawn _returnvalue))
    (Variables|Default|SetBase%20Pawn _asbp_base_pawn)))

(event EventTick
  (params (DeltaSeconds :type Float%20%28single-precision%29)))

(fn OnTakeAnyDamage
  (params (Damage :type Float%20%28double-precision%29))
  (bind _asbp_wg_health_bar (|SetHealthBarWidget))
  (|ChangeHealthPercentage _asbp_wg_health_bar Damage)
  (|DestroyActorIfHpReachesZero))