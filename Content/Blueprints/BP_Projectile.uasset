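; BP_Projectile is a projectile actor that damages turret pawns and expires beyond a maximum range.
; It records its start location when the ProjectileMovement component activates, then checks its straight-line distance from there every Tick.
; Collision hits apply damage only to actors whose class is exactly BP_PawnTurret; other hits are ignored.
; Both range expiry and turret hits call DestroyProjectile, which destroys the actor and spawns an auto-release pooled hit emitter.
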(event OnComponentHit(Collision)
  (params (HitComponent :type Primitive%20Component%20Object%20Reference) (OtherActor :type Actor%20Object%20Reference) (OtherComp :type Primitive%20Component%20Object%20Reference) (NormalImpulse :type Vector :default "0, 0, 0") (Hit :type Hit%20Result%20Structure%20%28by%20ref%29))
  (if (== (Utilities|GetClass OtherActor) "/Game/Blueprints/Pawns/BP_PawnTurret.BP_PawnTurret_C")
    (bind _asbp_pawn_turret (Utilities|Casting|CastToBP_PawnTurret OtherActor))
    (Game|Damage|ApplyDamage _asbp_pawn_turret 1.0 0 0)
    (CallFunction|EventDestroyProjectile (.impactpoint Hit))))

(event OnComponentActivated(ProjectileMovement)
  (params (Component :type Actor%20Component%20Object%20Reference) (bReset :type Boolean))
  ;[1 1 1] Set Initial Distance
  (Variables|Default|SetInitial%20Location (Transformation|GetWorldLocation (Variables|Default|GetCollision))))

(event Custom|Event%20Destroy%20Projectile
  (params (Location :type Vector))
  (Actor|DestroyActor)
  (Effects|SpawnEmitteratLocation "/Game/Assets/Effects/P_HitEffect.P_HitEffect" Location "0, 0, 0" "1.000000,1.000000,1.000000" true "AutoRelease"))

(event EventTick
  (params (DeltaSeconds :type Float%20%28single-precision%29))
  (bind _collision (Variables|Default|GetCollision))
  (bind _returnvalue (Transformation|GetWorldLocation _collision))
  ;[1 1 1] Destroy Based on Distance
  (if (> (Math|Vector|Distance(Vector) (Variables|Default|GetInitial%20Location) _returnvalue) (Variables|Default|GetMax%20Distance))
    (bind _output_get (Variables|Default|SetFinal%20Location _returnvalue))
    (CallFunction|EventDestroyProjectile _output_get)))

(fn ConstructionScript)