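; Player controller that drives the player's tank pawn from Enhanced Input movement actions.
; On BeginPlay it casts player pawn 0 to BP_PawnTank and caches the reference.
; While IA_Movement is triggered, the Y axis moves the tank along its local forward axis and the X axis adds yaw, scaled by the tank's MovementSpeed and RotationSpeed without delta time.
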(event Input|EnhancedActionEvents|EnhancedInputActionIA_Movement
  (params (ActionValue :type Vector%202D%20Structure) (ElapsedSeconds :type Float%20%28double-precision%29) (TriggeredSeconds :type Float%20%28double-precision%29) (InputAction :type Input%20Action%20Object%20Reference :default "/Game/Controller/IA_Movement.IA_Movement"))
  (bind _as_bp_pawn_tank (Variables|Default|GetAs%20BP%20Pawn%20Tank))
  (:Triggered
    (Transformation|AddActorLocalOffset _as_bp_pawn_tank (Math|Vector|MakeVector (* (.y ActionValue) (Variables|/Game/Blueprints/Pawns/BP_PawnTank.BP_PawnTank_C|GetMovement%20Speed _as_bp_pawn_tank)) 0.0 0.0) false false)
    (Transformation|SetActorRotation _as_bp_pawn_tank (Math|Rotator|MakeRotator 0.0 0.0 (+ (* (.x ActionValue) (Variables|/Game/Blueprints/Pawns/BP_PawnTank.BP_PawnTank_C|GetRotation%20Speed _as_bp_pawn_tank)) (.yaw (Transformation|GetActorRotation _as_bp_pawn_tank)))))))

(event EventBeginPlay
  ;[1 1 1] Begin
  (bind _asbp_pawn_tank (Utilities|Casting|CastToBP_PawnTank (Game|Player|GetPlayerPawn 0)))
  (Variables|Default|SetAs%20BP%20Pawn%20Tank _asbp_pawn_tank))

(fn ConstructionScript)